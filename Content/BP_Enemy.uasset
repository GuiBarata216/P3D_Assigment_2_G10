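; BP_Enemy is a roaming enemy that hunts the player and destroys the player character on reaching it.
; It wanders by chaining AI moves to random navigable points within a radius, repeating on each success.
; When PawnSensing sees any pawn, it sets its walk speed, flags the sighting permanently and moves toward player 0.
; A breakObject event destroys the enemy itself.
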(event OnSeePawn(PawnSensing)
  (params (Pawn :type Pawn%20Object%20Reference))
  (Variables|/Script/Engine.CharacterMovementComponent|SetMaxWalkSpeed (Variables|Character|GetCharacterMovement) 4e+02)
  (Variables|Default|SetisSeingPlayer true)
  (CallFunction|FollowPlayer))

(event Custom|Follow%20Player
  (if (Variables|Default|GetisSeingPlayer)
    (AI|AIMoveTo self "0, 0, 0" (Game|GetPlayerCharacter 0) 15.0 false
      (:OnSuccess
        (Actor|DestroyActor (Game|GetPlayerCharacter 0))))))

(event Custom|breakObject
  (Actor|DestroyActor))

(event Custom|moveRandom
  (bind _randomlocation (Class|NavigationSystemV1|GetRandomLocationinNavigableRadius (Transformation|GetActorLocation) 1.5e+03 0 0))
  (AI|AIMoveTo self _randomlocation 0 5.0 false
    (:OnSuccess
      (CallFunction|MoveRandom))))

(event EventBeginPlay
  (CallFunction|MoveRandom))

(fn ConstructionScript)